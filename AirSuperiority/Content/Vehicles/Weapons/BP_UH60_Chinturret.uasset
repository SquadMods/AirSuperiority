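; Chin turret vehicle weapon Blueprint for the UH-60 helicopter, handling its mounted position and camera zoom.
; On BeginPlay it snaps to a fixed relative offset and activates its Camera.
; Zooming uses a timeline to ease the first-person camera toward the user's FOV setting divided by the current zoom level.
; Resetting zoom restores base FOV on both cameras, switches to the first-person camera and clears the zoom index.
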(event `self.ReceiveBeginPlay`
  (`parent.ReceiveBeginPlay`)
  (`self.K2_SetActorRelativeLocation` (135.0 58.5 -68.0))
  (`ActorComponent.SetActive` (`self.Camera`) true false))

(event `self.BP_OnVehicleZoom`
  (bind _firstpersoncamera (`self.FirstPersonCamera`))
  ;[0 0.685 0.1713] ZoomEvents
  (bind (_direction _lerp) (`Timeline|Timeline_1`)
    (:`Update`
      (`CameraComponent.SetFieldOfView` _firstpersoncamera (`KismetMathLibrary.Lerp` (`CameraComponent.FieldOfView` _firstpersoncamera) (/ (`SQGameUserSettings.FOV` (`SQBlueprintLibrary.GetSquadGameUserSettings`)) (`|GetArrayItem` (`self.ZoomLevels`) (`self.CurrentZoom`))) _lerp)))))

(event `self.ResetZoom`
  ;[0 0.685 0.1713] ZoomEvents
  (`CameraComponent.SetFieldOfView` (`self.FirstPersonCamera`) (/ (`SQGameUserSettings.FOV` (`SQBlueprintLibrary.GetSquadGameUserSettings`)) (`|GetArrayItem` (`self.ZoomLevels`))))
  (`CameraComponent.SetFieldOfView` (`self.Camera`) (/ (`SQGameUserSettings.FOV` (`SQBlueprintLibrary.GetSquadGameUserSettings`)) (`|GetArrayItem` (`self.ZoomLevels`))))
  (`ActorComponent.SetActive` (`self.Camera`) false false)
  (`ActorComponent.SetActive` (`self.FirstPersonCamera`) true false)
  (set `self.CurrentZoom` 0))

(fn `UserConstructionScript`
  (`parent.UserConstructionScript`))