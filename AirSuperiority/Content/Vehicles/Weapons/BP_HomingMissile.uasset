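; BP_HomingMissile is a homing missile vehicle weapon that handles impacts differently depending on how long it has been in flight.
; Impacts at or before the minimum flight time spawn an attached effect and a loud, pitched-down sound on the skeletal mesh, skipping the parent's impact logic.
; Later impacts defer to the parent class, and no homing logic appears in this Blueprint.
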(event `self.ReceiveBeginPlay`)

(event `self.OnImpact`
  (params (SelfActor :type "Actor Object Reference") (OtherActor :type "Actor Object Reference") (NormalImpulse :type "Vector Structure") (Hit :type "HitResult Structure (by ref)"))
  (bind _skeletalmesh (`self.SkeletalMesh`))
  ;[1 1 1] BP Effect and Audio under minimum flight time
  (if (<= (`self.GetGameTimeSinceCreation` SelfActor) (`self.MinFlightTime`))
    (`GameplayStatics.SpawnEmitterAttached` (`self.BPEffectOnUnderMinFlightTime`) _skeletalmesh)
    (bind _returnvalue (`GameplayStatics.SpawnSoundAttached` (`self.BPSoundonUnderMinFlightTime`) _skeletalmesh "None" (0.0 0.0 0.0) (struct) "KeepRelativeOffset" false 3.0 0.3 0.0 "/Game/Audio/Attenuation/RPG/RPGCloseAttenuation.RPGCloseAttenuation" "/Game/Audio/Concurrency/BhitConcurrency.BhitConcurrency"))
    (`AudioComponent.Play` _returnvalue 0.0)
    (else
      (`parent.OnImpact` SelfActor OtherActor NormalImpulse Hit))))

(fn `UserConstructionScript`
  (`parent.UserConstructionScript`))