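; Vehicle missile launcher weapon with zoomed aiming, equip animations and a backblast on fire.
; Zooming with a valid reticle class shows a HUD overlay, narrows the SPG-9 technical turret camera to a quarter of user FOV and plays a timeline; unzooming or unpossessing reverts this.
; Equipping either plays tripod, weapon and soldier animations with input locked and the camera on the soldier, or starts a reload when empty.
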(event `self.BlueprintOnZoom`
  (params (bNewZoom :type Boolean))
  (bind _reticleclass (`self.ReticleClass`))
  (bind _returnvalue (`Pawn.GetController` (`self.GetOwnerSeat`)))
  (bind _returnvalue_2 (`Controller.K2_GetPawn` (`self.Last PC`)))
  (bind _fov (`SQGameUserSettings.FOV` (`SQBlueprintLibrary.GetSquadGameUserSettings`)))
  ;[0 0 0] ADS, change FOV and apply post processing
  (`parent.BlueprintOnZoom` bNewZoom)
  (`/Engine/EditorBlueprintResources/StandardMacros.Can Execute Cosmetic Events`
    (:`True`
      (set `self.Last PC` _returnvalue)
      (bind _assqplayer_controller (cast `SQPlayerController` _returnvalue))
      (bind _assqhud (cast `SQHUD` (`PlayerController.GetHUD` _assqplayer_controller)))
      (set `self.Last HUD` _assqhud)
      (if bNewZoom
        (if (`KismetSystemLibrary.IsValidClass` _reticleclass)
          (`SQHUD.VehicleCreateOverlay` _assqhud _reticleclass)
          (bind _asbp_technical_turret_spg9 (cast `/Game/Vehicles/Technical/BP_Technical_Turret_SPG9` _returnvalue_2))
          (`CameraComponent.SetFieldOfView` (`/Game/Vehicles/BP_GenericVehicleOpenTurret.Camera1pComponent` _asbp_technical_turret_spg9) (/ _fov 4.0))
          (`Timeline|Timeline_0` :!label _label)
          (else
            (`SQHUD.VehicleRemoveOverlay` (stale `RemoveADS` _last_hud) null :!label _label_2)
            (bind _asbp_technical_turret_spg9_2 (cast `/Game/Vehicles/Technical/BP_Technical_Turret_SPG9` _returnvalue_2))
            (`CameraComponent.SetFieldOfView` (`/Game/Vehicles/BP_GenericVehicleOpenTurret.Camera1pComponent` _asbp_technical_turret_spg9_2) _fov)
            (goto _label :!via `Stop`)))
        (else
          (goto _label_2))))))

(event `RemoveADS`
  ;[0 0 0] ADS, change FOV and apply post processing
  (bind _last_hud (`self.Last HUD`)
    (:`then`
      (goto _label_2))
    (:`else`)))

(event `self.ReceiveBeginPlay`
  ;[0 0 0] ADS, change FOV and apply post processing
  (`KismetSystemLibrary.Delay` 1.0)
  (bind _assqpawn (cast `SQPawn` (`self.GetOwnerPawn`)))
  (add `SQPawn.OnPawnPossessedEvent` _assqpawn (delegate `CPossessed`))
  (add `SQPawn.OnPawnUnPossessedEvent` _assqpawn (delegate `CUnpossessed`)))

(event `CUnpossessed`
  ;[0 0 0] ADS, change FOV and apply post processing
  (`self.RemoveADS`))

(event `CPossessed`
  ;[0 0 0] ADS, change FOV and apply post processing
)

(event `self.BlueprintOnEquip`
  ;[1 1 1] Fire and Equip Animations
  (set `self.bIgnoreCameraChange` false)
  (`/Engine/EditorBlueprintResources/StandardMacros.IsValid` (`self.GetSoldier`)
    (:`Is Valid`
      (if (`self.MagazineHasAmmo`)
        (`self.CameraOnSoldier`)
        (set `self.bInputEnabled` false)
        (bind (_tripodanimtime _weaponanimtime) (`self.PlayAnimations` (`self.Equip Tripod Animation`) (`self.Equip Weapon Animation`) (`self.Equip Soldier Animation`)))
        (`KismetSystemLibrary.RetriggerableDelay` _weaponanimtime)
        (set `self.bInputEnabled` true)
        (`self.CameraOnWeapon`)
        (else
          (`self.StartReload`))))))

(event `self.BlueprintOnFire`
  (params (Origin :type "Vector Structure (by ref)"))
  ;[1 1 1] Fire and Equip Animations
  ;;[1 1 1] Play SQBlast (Backblast) on Fire
  (`parent.BlueprintOnFire` Origin)
  (`/Engine/EditorBlueprintResources/StandardMacros.Can Execute Cosmetic Events`
    (:`True`
      (`SQBlastComponent.FireBlast` (`self.SQBlast`)))))

(fn `UserConstructionScript`
  (bind _sqblast (`self.SQBlast`))
  (set `SceneComponent.bAbsoluteScale` true _sqblast)
  (`SceneComponent.K2_AttachToComponent` _sqblast (`self.Mesh3P`) (`self.BackblastSocket`) "SnapToTarget" "SnapToTarget" "KeepWorld" true))