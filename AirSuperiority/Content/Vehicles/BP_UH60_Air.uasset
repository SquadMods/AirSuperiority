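; UH-60 helicopter vehicle Blueprint that adds a toggleable in-cockpit music radio and pilot camera zoom, and repositions the current weapon on BeginPlay.
; Ctrl+Alt+Shift+P toggles the radio, choosing a playlist and random song, with a looping timer for autoplay checks.
; P, O and I switch between all, Vietnam and meme playlists and step tracks, while Add/Subtract adjust volume.
; PilotZoom interpolates camera FOV, plus pitch outside free look.
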(event `self.ReceiveBeginPlay`
  (bind _currentweapon (`SQPawnInventoryComponent.CurrentWeapon` (`self.SQVehicleResourceWeaponInventory`)))
  ;[1 1 1] Set SongLists
  (`parent.ReceiveBeginPlay`)
  (bind _output_get (set `self.Song_List_All` (`|MakeArray` "/AirSuperiority/Assets/Audio/RadioSongs/Ouija.Ouija" "/AirSuperiority/Assets/Audio/RadioSongs/BeeHiveYourself.BeeHiveYourself" "/AirSuperiority/Assets/Audio/RadioSongs/WeGotThePower.WeGotThePower" "/AirSuperiority/Assets/Audio/RadioSongs/StrangeGalaxy.StrangeGalaxy" "/AirSuperiority/Assets/Audio/RadioSongs/TheConnection.TheConnection" "/AirSuperiority/Assets/Audio/RadioSongs/CremeSupreme.CremeSupreme" "/AirSuperiority/Assets/Audio/RadioSongs/RideOfTheValkyries.RideOfTheValkyries" "/AirSuperiority/Assets/Audio/RadioSongs/VillageStrollin.VillageStrollin" "/AirSuperiority/Assets/Audio/RadioSongs/RunThroughtheJungle.RunThroughtheJungle" "/AirSuperiority/Assets/Audio/RadioSongs/FortunateSon.FortunateSon" "/AirSuperiority/Assets/Audio/RadioSongs/ACountryDance.ACountryDance" "/AirSuperiority/Assets/Audio/RadioSongs/Superstition.Superstition" "/AirSuperiority/Assets/Audio/RadioSongs/FeelsSoGood.FeelsSoGood" "/AirSuperiority/Assets/Audio/RadioSongs/TakeFive.TakeFive" "/AirSuperiority/Assets/Audio/RadioSongs/Wndrwll.Wndrwll" "/AirSuperiority/Assets/Audio/RadioSongs/SexualLionKing.SexualLionKing" "/AirSuperiority/Assets/Audio/RadioSongs/advertisement1.advertisement1" "/AirSuperiority/Assets/Audio/RadioSongs/SayItAintSoCal.SayItAintSoCal" "/AirSuperiority/Assets/Audio/RadioSongs/TIME.TIME" "/AirSuperiority/Assets/Audio/RadioSongs/AVDC.AVDC" "/AirSuperiority/Assets/Audio/RadioSongs/HotDrinks.HotDrinks" "/AirSuperiority/Assets/Audio/RadioSongs/RideTheTrain.RideTheTrain" "/AirSuperiority/Assets/Audio/RadioSongs/DangerZone.DangerZone" "/AirSuperiority/Assets/Audio/RadioSongs/advertisement2.advertisement2" "/AirSuperiority/Assets/Audio/RadioSongs/Sandstorm.Sandstorm" "/AirSuperiority/Assets/Audio/RadioSongs/Reptillia.Reptillia" "/AirSuperiority/Assets/Audio/RadioSongs/CarryOn.CarryOn" "/AirSuperiority/Assets/Audio/RadioSongs/CarryOn.CarryOn" "/AirSuperiority/Assets/Audio/RadioSongs/PleaseUseThis.PleaseUseThis" "/AirSuperiority/Assets/Audio/RadioSongs/TokuSentai.TokuSentai" "/AirSuperiority/Assets/Audio/RadioSongs/advertisement3.advertisement3" "/AirSuperiority/Assets/Audio/RadioSongs/DejaVu.DejaVu" "/AirSuperiority/Assets/Audio/RadioSongs/DoggyBounce.DoggyBounce" "/AirSuperiority/Assets/Audio/RadioSongs/BadCompany.BadCompany" "/AirSuperiority/Assets/Audio/RadioSongs/BeatIt.BeatIt" "/AirSuperiority/Assets/Audio/RadioSongs/WowWow.WowWow" "/AirSuperiority/Assets/Audio/RadioSongs/DissinYourFlyGirl.DissinYourFlyGirl" "/AirSuperiority/Assets/Audio/RadioSongs/USA2.USA2" "/AirSuperiority/Assets/Audio/RadioSongs/APM.APM" "/AirSuperiority/Assets/Audio/RadioSongs/ComeFlyWithMe.ComeFlyWithMe" "/AirSuperiority/Assets/Audio/RadioSongs/advertisement4.advertisement4" "/AirSuperiority/Assets/Audio/RadioSongs/GuitarSoul.GuitarSoul" "/AirSuperiority/Assets/Audio/RadioSongs/SurfHoundDay.SurfHoundDay" "/AirSuperiority/Assets/Audio/RadioSongs/Scramble.Scramble" "/AirSuperiority/Assets/Audio/RadioSongs/PictureOfSpring.PictureOfSpring" "/AirSuperiority/Assets/Audio/RadioSongs/FlowerPower.FlowerPower" "/AirSuperiority/Assets/Audio/RadioSongs/RhythmUnderTheSkin.RhythmUnderTheSkin" "/AirSuperiority/Assets/Audio/RadioSongs/MuscleSoul.MuscleSoul" "/AirSuperiority/Assets/Audio/RadioSongs/HesOnFireworks.HesOnFireworks" "/AirSuperiority/Assets/Audio/RadioSongs/DavidCameronRap.DavidCameronRap" "/AirSuperiority/Assets/Audio/RadioSongs/PunchYouInTheJeans.PunchYouInTheJeans" :!type "SoundBase Object Reference")))
  (`KismetArrayLibrary.Array_Shuffle` _output_get)
  (set `self.Song_List_Vietnam` (`|MakeArray` "/AirSuperiority/Assets/Audio/RadioSongs/Ouija.Ouija" "/AirSuperiority/Assets/Audio/RadioSongs/BeeHiveYourself.BeeHiveYourself" "/AirSuperiority/Assets/Audio/RadioSongs/WeGotThePower.WeGotThePower" "/AirSuperiority/Assets/Audio/RadioSongs/StrangeGalaxy.StrangeGalaxy" "/AirSuperiority/Assets/Audio/RadioSongs/TheConnection.TheConnection" "/AirSuperiority/Assets/Audio/RadioSongs/CremeSupreme.CremeSupreme" "/AirSuperiority/Assets/Audio/RadioSongs/RideOfTheValkyries.RideOfTheValkyries" "/AirSuperiority/Assets/Audio/RadioSongs/VillageStrollin.VillageStrollin" "/AirSuperiority/Assets/Audio/RadioSongs/RunThroughtheJungle.RunThroughtheJungle" "/AirSuperiority/Assets/Audio/RadioSongs/FortunateSon.FortunateSon" "/AirSuperiority/Assets/Audio/RadioSongs/Superstition.Superstition" "/AirSuperiority/Assets/Audio/RadioSongs/BadCompany.BadCompany" "/AirSuperiority/Assets/Audio/RadioSongs/ComeFlyWithMe.ComeFlyWithMe" "/AirSuperiority/Assets/Audio/RadioSongs/GuitarSoul.GuitarSoul" "/AirSuperiority/Assets/Audio/RadioSongs/SurfHoundDay.SurfHoundDay" "/AirSuperiority/Assets/Audio/RadioSongs/Scramble.Scramble" "/AirSuperiority/Assets/Audio/RadioSongs/PictureOfSpring.PictureOfSpring" "/AirSuperiority/Assets/Audio/RadioSongs/FlowerPower.FlowerPower" "/AirSuperiority/Assets/Audio/RadioSongs/RhythmUnderTheSkin.RhythmUnderTheSkin" "/AirSuperiority/Assets/Audio/RadioSongs/MuscleSoul.MuscleSoul" :!type "SoundBase Object Reference"))
  (set `self.Song_List_Memes` (`|MakeArray` "/AirSuperiority/Assets/Audio/RadioSongs/ACountryDance.ACountryDance" "/AirSuperiority/Assets/Audio/RadioSongs/FeelsSoGood.FeelsSoGood" "/AirSuperiority/Assets/Audio/RadioSongs/TakeFive.TakeFive" "/AirSuperiority/Assets/Audio/RadioSongs/Wndrwll.Wndrwll" "/AirSuperiority/Assets/Audio/RadioSongs/SexualLionKing.SexualLionKing" "/AirSuperiority/Assets/Audio/RadioSongs/SayItAintSoCal.SayItAintSoCal" "/AirSuperiority/Assets/Audio/RadioSongs/TIME.TIME" "/AirSuperiority/Assets/Audio/RadioSongs/AVDC.AVDC" "/AirSuperiority/Assets/Audio/RadioSongs/HotDrinks.HotDrinks" "/AirSuperiority/Assets/Audio/RadioSongs/RideTheTrain.RideTheTrain" "/AirSuperiority/Assets/Audio/RadioSongs/DangerZone.DangerZone" "/AirSuperiority/Assets/Audio/RadioSongs/Sandstorm.Sandstorm" "/AirSuperiority/Assets/Audio/RadioSongs/Reptillia.Reptillia" "/AirSuperiority/Assets/Audio/RadioSongs/CarryOn.CarryOn" "/AirSuperiority/Assets/Audio/RadioSongs/PleaseUseThis.PleaseUseThis" "/AirSuperiority/Assets/Audio/RadioSongs/TokuSentai.TokuSentai" "/AirSuperiority/Assets/Audio/RadioSongs/DejaVu.DejaVu" "/AirSuperiority/Assets/Audio/RadioSongs/DoggyBounce.DoggyBounce" "/AirSuperiority/Assets/Audio/RadioSongs/BeatIt.BeatIt" "/AirSuperiority/Assets/Audio/RadioSongs/WowWow.WowWow" "/AirSuperiority/Assets/Audio/RadioSongs/DissinYourFlyGirl.DissinYourFlyGirl" "/AirSuperiority/Assets/Audio/RadioSongs/USA2.USA2" "/AirSuperiority/Assets/Audio/RadioSongs/APM.APM" "/AirSuperiority/Assets/Audio/RadioSongs/ComeFlyWithMe.ComeFlyWithMe" "/AirSuperiority/Assets/Audio/RadioSongs/HesOnFireworks.HesOnFireworks" "/AirSuperiority/Assets/Audio/RadioSongs/DavidCameronRap.DavidCameronRap" "/AirSuperiority/Assets/Audio/RadioSongs/PunchYouInTheJeans.PunchYouInTheJeans" :!type "SoundBase Object Reference"))
  (`self.K2_SetActorRelativeRotation` _currentweapon (struct :`Pitch` -4.7) false false)
  (`self.K2_SetActorRelativeLocation` _currentweapon (285.0 158.0 103.0) false false))

(event `ShouldPlayNextSong`
  ;[1 1 1] Helicopter Radio
  (`KismetSystemLibrary.PrintString` "It works")
  (if (`AudioComponent.IsPlaying` (`self.Heli_Radio_Songs`))
    _
    (elif (`ActorComponent.IsActive` (`self.Scene`))
      (`self.Next Song Random`))))

(event `Key|Ctrl+Alt+Shift+P`
  (params (Key :type "Key Structure"))
  (bind _nowplaying (`self.NowPlaying`))
  (bind _heli_radio_songs (`self.Heli_Radio_Songs`))
  (bind _scene (`self.Scene`))
  (bind _heli_radio_chh (`self.Heli_Radio_Chh`))
  (bind _songname (`self.SongName`))
  (:`Pressed`
    (`/Engine/EditorBlueprintResources/StandardMacros.FlipFlop`
      (:`A`
        (`AudioComponent.Play` _heli_radio_chh 0.0)
        (`TextRenderComponent.K2_SetText` _nowplaying (`KismetTextLibrary.Conv_StringToText` "Radio On <br>Now Playing"))
        (`ActorComponent.Activate` _heli_radio_songs false)
        (`ActorComponent.Activate` _scene false)
        (`TextRenderComponent.K2_SetText` _songname (`KismetTextLibrary.Conv_StringToText` "None"))
        (`SceneComponent.SetVisibility` _songname true false)
        (switch `int` (`KismetMathLibrary.RandomInteger` 2)
          (:`0`
            (set `self.Song_List_Current` (`self.Song_List_Vietnam`)))
          (:`1`
            (set `self.Song_List_Current` (`self.Song_List_Memes`)))
          (:`2`
            (set `self.Song_List_Current` (`self.Song_List_All`))))
        (if (`ActorComponent.IsActive` (`self.Scene`))
          (`self.Next Song Random`)
          (bind _returnvalue (`KismetSystemLibrary.K2_SetTimerDelegate` (`|CreateDelegate` :!event `ShouldPlayNextSong`) 5.0 true))
          (set `self.Radio_Check` _returnvalue)))
      (:`B`
        (`AudioComponent.Play` _heli_radio_chh 0.0)
        (`TextRenderComponent.K2_SetText` _nowplaying (`KismetTextLibrary.Conv_StringToText` "Radio Off<br>Turn it On!"))
        (`ActorComponent.Deactivate` _heli_radio_songs)
        (`ActorComponent.Deactivate` _scene)
        (`AudioComponent.Stop` (`self.Heli_Radio_Songs`))
        (`SceneComponent.SetVisibility` _songname false false)
        (`KismetSystemLibrary.K2_ClearAndInvalidateTimerHandle` (`self.Radio_Check`))))))

(event `Key|P`
  (params (Key :type "Key Structure"))
  ;[1 1 1] Helicopter Radio
  (:`Pressed`
    (set `self.Song_List_Current` (`self.Song_List_All`))
    (if (`ActorComponent.IsActive` (`self.Scene`))
      (`self.NextSongInList` (`self.CheckListLength`)))))

(event `Key|O`
  (params (Key :type "Key Structure"))
  ;[1 1 1] Helicopter Radio
  (:`Pressed`
    (set `self.Song_List_Current` (`self.Song_List_Vietnam`))
    (if (`ActorComponent.IsActive` (`self.Scene`))
      (`self.NextSongInList` (`self.CheckListLength`)))))

(event `Key|I`
  (params (Key :type "Key Structure"))
  ;[1 1 1] Helicopter Radio
  (:`Pressed`
    (set `self.Song_List_Current` (`self.Song_List_Memes`))
    (if (`ActorComponent.IsActive` (`self.Scene`))
      (`self.NextSongInList` (`self.CheckListLength`)))))

(event `self.PilotZoom`
  (params (InputPin :type "Float (single-precision)"))
  (bind _returnvalue (`KismetMathLibrary.FClamp` InputPin -1.0 0.0))
  (bind _pilotcamera (`self.PilotCamera`))
  ;[1 1 1] Zoom
  (if (not (`SQFreeLookComponent.GetIsUsingFreeLook` (`self.FreeLookComponent`)))
    (`SceneComponent.K2_SetRelativeRotation` _pilotcamera (`KismetMathLibrary.RInterpTo` (`SceneComponent.RelativeRotation` (`self.PilotCamera`)) (`KismetMathLibrary.RLerp` (struct :`Pitch` -5.0) (`KismetMathLibrary.ComposeRotators` (struct :`Pitch` -5.0) (`self.Pilot-ZoomCameraRotation`)) _returnvalue) (`GameplayStatics.GetWorldDeltaSeconds`) 8.0) false false))
  (`CameraComponent.SetFieldOfView` _pilotcamera (`KismetMathLibrary.FInterpTo` (`CameraComponent.FieldOfView` _pilotcamera) (`KismetMathLibrary.Lerp` 100.0 165.0 _returnvalue) (`GameplayStatics.GetWorldDeltaSeconds`) 8.0)))

(event `Key|Add`
  (params (Key :type "Key Structure"))
  (bind _volumemultiplier (`AudioComponent.VolumeMultiplier` (`self.Heli_Radio_Songs`)))
  ;[1 1 1] Adjust Volume
  (:`Pressed`
    (if (`ActorComponent.IsActive` (`self.Scene`))
      (if (< _volumemultiplier 2.0)
        (`AudioComponent.SetVolumeMultiplier` (`self.Heli_Radio_Songs`) (+ 0.1 _volumemultiplier))
        (`KismetSystemLibrary.PrintString` (`KismetStringLibrary.Conv_DoubleToString` _volumemultiplier))))))

(event `Next Song Random`
  ;[1 1 1] Next Song AutoPlay
  (if (`ActorComponent.IsActive` (`self.Scene`))
    (`self.RandomSongAutoPlay`)))

(event `Key|Subtract`
  (params (Key :type "Key Structure"))
  (bind _volumemultiplier (`AudioComponent.VolumeMultiplier` (`self.Heli_Radio_Songs`)))
  ;[1 1 1] Adjust Volume
  (:`Pressed`
    (if (`ActorComponent.IsActive` (`self.Scene`))
      (if (> _volumemultiplier 0.1)
        (`AudioComponent.SetVolumeMultiplier` (`self.Heli_Radio_Songs`) (- _volumemultiplier 0.1))
        (`KismetSystemLibrary.PrintString` (`KismetStringLibrary.Conv_DoubleToString` _volumemultiplier))))))

(fn `NextSongInList`
  (params (Condition :type Boolean))
  (bind _songname (`self.SongName`))
  (bind _song_list_current (`self.Song_List_Current`))
  (bind _heli_radio_songs (`self.Heli_Radio_Songs`))
  (`AudioComponent.Play` (`self.Heli_Radio_Chh`) 0.0)
  (if Condition
    (bind _output_get (set `self.CurrentTrack` 0))
    (bind _output (`|GetArrayItem` _song_list_current _output_get))
    (`AudioComponent.SetSound` _heli_radio_songs _output)
    (`AudioComponent.Play` _heli_radio_songs 0.0)
    (`TextRenderComponent.K2_SetText` _songname (`KismetTextLibrary.Conv_StringToText` (`KismetSystemLibrary.GetObjectName` _output)))
    (else
      (bind _result (`/Engine/EditorBlueprintResources/StandardMacros.IncrementInt` (`self.CurrentTrack`))
        (:`  `
          (bind _output_2 (`|GetArrayItem` _song_list_current _result))
          (`AudioComponent.SetSound` _heli_radio_songs _output_2)
          (`AudioComponent.Play` _heli_radio_songs 0.0)
          (`TextRenderComponent.K2_SetText` _songname (`KismetTextLibrary.Conv_StringToText` (`KismetSystemLibrary.GetObjectName` _output_2))))))))

(fn `RandomSongAutoPlay`
  (bind _heli_radio_songs (`self.Heli_Radio_Songs`))
  (`AudioComponent.SetSound` _heli_radio_songs (`|GetArrayItem` (`self.Song_List_Current`) (`KismetMathLibrary.RandomIntegerInRange` 0 (`KismetArrayLibrary.Array_Length` (`self.Song_List_Current`)))))
  (`AudioComponent.Play` _heli_radio_songs 0.0)
  (`TextRenderComponent.K2_SetText` (`self.SongName`) (`KismetTextLibrary.Conv_StringToText` (`KismetSystemLibrary.GetObjectName` (`AudioComponent.Sound` _heli_radio_songs)))))

(fn `UserConstructionScript`
  (`parent.UserConstructionScript`))