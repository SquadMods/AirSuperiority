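; An explodable tank prop, named for Squad mortar fire, that detonates when a mortar projectile overlaps its capsule.
; After a short delay it activates its particle effect and applies large-radius heat damage with falloff from that point on the Destructible prevention channel.
; All soldier actors are passed as ignored, so the blast spares infantry.
; The tank mesh is then hidden and collision is disabled rather than destroying the actor.
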(event `self.Capsule.OnComponentBeginOverlap`
  (params (OverlappedComponent :type "PrimitiveComponent Object Reference") (OtherActor :type "Actor Object Reference") (OtherComp :type "PrimitiveComponent Object Reference") (OtherBodyIndex :type Integer) (bFromSweep :type Boolean) (SweepResult :type "HitResult Structure (by ref)"))
  (if (`KismetMathLibrary.ClassIsChildOf` (`GameplayStatics.GetObjectClass` OtherActor) "/Script/Squad.SQMortarProjectile")
    (`KismetSystemLibrary.Delay` 0.2)
    (`ActorComponent.Activate` (`self.ParticleSystem`) false)
    (bind _outactors (`GameplayStatics.GetAllActorsOfClass` "/Script/Squad.SQSoldierNew"))
    (`GameplayStatics.ApplyRadialDamageWithFalloff` 1250.0 0.0 (`SceneComponent.K2_GetComponentLocation` (`self.ParticleSystem`)) 2000.0 17500.0 2.0 "/Game/Gameplay/DamageTypes/BP_BasicHeatDamageType.BP_BasicHeatDamageType_C" _outactors null null "ECC_Destructible")
    (`KismetSystemLibrary.Delay` 0.1)
    (`SceneComponent.SetVisibility` (`self.Tank`) false false)
    (`PrimitiveComponent.SetCollisionEnabled` (`self.Tank`) "NoCollision")
    (`PrimitiveComponent.SetCollisionEnabled` (`self.Capsule`) "NoCollision")))

(fn `UserConstructionScript`)